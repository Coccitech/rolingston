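; Player rolling-ball pawn that grows as it accumulates travelled distance and shows a death screen with mouse cursor when destroyed.
; Axis inputs apply velocity-change impulses on X and Y.
; Self-recursing Delay loops drive AddDistance, which scales the ball toward the last BallTier value and records its tier, and Cameramove, which offsets the camera by scale up to a limit.
; An X speed limiter is defined but nothing here starts it.
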(event `self.ReceiveDestroyed`
  ;[1 1 1] HUD Mort
  (bind _returnvalue (`|CreateWidget` "/Game/BluePrint/HUD_DeathScreen.HUD_DeathScreen_C"))
  (`UserWidget.AddToViewport` _returnvalue 0)
  (set `PlayerController.bShowMouseCursor` true (`GameplayStatics.GetPlayerController` 0)))

(event `self.ReceiveBeginPlay`
  ;[1 1 1] Sphere Scale, Location & Distance
  (`self.K2_SetActorLocation` (0.0 0.0 0.0) false true)
  (set `self.sphereLocation` (`self.K2_GetActorLocation`))
  (bind _output_get (set `self.sphereScale` (`self.GetActorScale3D`)))
  (`self.Add Distance`)
  (`self.Cameramove`))

(event `InputAxis|Avant/Arrière`
  (params (AxisValue :type "Float (single-precision)"))
  (bind _vitessex (`self.vitesseX`))
  ;[1 1 1] Ball Movement X
  (if (<= _vitessex (`self.vitesseMaxX`))
    (`PrimitiveComponent.AddImpulse` (`self.Sphere`) (* (`KismetMathLibrary.MakeVector` AxisValue) _vitessex) "None" true)))

(event `Add Distance`
  (bind _balltier (`self.ballTier`))
  (bind _spheredistance (`self.sphereDistance`))
  (bind _returnvalue_x (`KismetMathLibrary.BreakVector` (+ (`self.sphereLocation`) (375000.0 0.0 0.0))))
  ;[1 1 1] Sphere Scale, Location & Distance
  (set `self.sphereDistance` (+ _spheredistance (* (`KismetMathLibrary.VSize` (`self.GetVelocity`)) (`GameplayStatics.GetWorldDeltaSeconds`))))
  (bind _keys (`BlueprintMapLibrary.Map_Keys` _balltier))
  (bind _values (`BlueprintMapLibrary.Map_Values` _balltier))
  (for _array_element _keys
    (if (> (stale _output_get_2) (`BlueprintMapLibrary.Map_Find` _balltier _array_element))
      (bind _output_get (set `self.currentTierancien` _array_element))))
  (bind _returnvalue (`KismetMathLibrary.Lerp` 1.0 (`|GetArrayItem` _values (`KismetArrayLibrary.Array_LastIndex` _values)) (`KismetMathLibrary.MapRangeClamped` _spheredistance 0.0 _returnvalue_x 0.0 1.0)))
  (`self.SetActorScale3D` (* (stale `self.ReceiveBeginPlay` _output_get) _returnvalue))
  (bind _output_get_2 (set `self.scaleFactor` _returnvalue))
  (bind _output_get_3 (set `self.springArmLenght` (- (`KismetMathLibrary.VSize` (`SceneComponent.K2_GetComponentLocation` (`self.Camera`))) (`KismetMathLibrary.VSize` (`SceneComponent.K2_GetComponentLocation` (`self.Sphere`))))))
  (bind _output_get_4 (set `self.scaleRate` (/ (- 50.0 _output_get_3) _output_get_3)))
  (`KismetSystemLibrary.PrintString` (`KismetStringLibrary.Conv_DoubleToString` _output_get_3))
  (`KismetSystemLibrary.Delay` _output_get_4)
  (`self.Add Distance`))

(event `InputAxis|Gauche/Droite`
  (params (AxisValue :type "Float (single-precision)"))
  (bind _vitessey (`self.vitesseY`))
  ;[1 1 1] Ball Movement Y
  (if (<= _vitessey (`self.vitesseMaxY`))
    (`PrimitiveComponent.AddImpulse` (`self.Sphere`) (* (`KismetMathLibrary.MakeVector` 0.0 AxisValue) _vitessey) "None" true)))

(event `LimitateurVitesse`
  (bind _returnvalue_x (`KismetMathLibrary.BreakVector` (`self.GetVelocity`)))
  (bind _vitessemaxx (`self.vitesseMaxX`))
  ;[1 1 1] Limitateur vitesse
  (if (not (<= _returnvalue_x _vitessemaxx))
    (`PrimitiveComponent.AddImpulse` (`self.Sphere`) (`KismetMathLibrary.MakeVector` (- _vitessemaxx _returnvalue_x)) "None" true)
    (`KismetSystemLibrary.Delay` 0.0004)
    (`self.LimitateurVitesse`)))

(event `Cameramove`
  (bind _scalerate (`self.scaleRate`))
  (bind _scalefactor (`self.scaleFactor`))
  (bind _returnvalue_x (`KismetMathLibrary.BreakVector` (* (* (`SceneComponent.K2_GetComponentScale` (`self.SpringArm`)) _scalefactor) _scalerate)))
  (if (<= _scalefactor 16.0)
    (`SceneComponent.K2_SetRelativeLocation` (`self.Camera`) (`KismetMathLibrary.MakeVector` _returnvalue_x 0.0 (* _scalefactor (`KismetMathLibrary.Abs` _scalerate))) false true)
    (`KismetSystemLibrary.Delay` 0.0004)
    (`self.Cameramove`)))

(fn `UserConstructionScript`)