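; BP_obstTier3 is an obstacle actor that tests the tier of any player overlapping its collision.
; If the obstacle's tier is at or below the player's CurrentTier, its cylinder starts simulating physics and takes an impulse from the player's velocity, then the actor is destroyed after a short delay.
; Otherwise the player actor is destroyed.
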(event `self.Collision.OnComponentBeginOverlap`
  (params (OverlappedComponent :type "PrimitiveComponent Object Reference") (OtherActor :type "Actor Object Reference") (OtherComp :type "PrimitiveComponent Object Reference") (OtherBodyIndex :type Integer) (bFromSweep :type Boolean) (SweepResult :type "HitResult Structure (by ref)"))
  (bind _asbp_player (cast `/Game/BluePrint/BP_Player` OtherActor))
  (bind _output_get (set `self.As BP Player` _asbp_player))
  (if (<= (`self.currentTierObst`) (`/Game/BluePrint/BP_Player.currentTier` _output_get))
    (`PrimitiveComponent.SetSimulatePhysics` (`self.Cylinder`) true)
    (`PrimitiveComponent.AddImpulse` (`self.Cylinder`) (`self.GetVelocity` (`self.As BP Player`)) "None" true)
    (`KismetSystemLibrary.Delay` 5.0)
    (`self.K2_DestroyActor`)
    (else
      (`self.K2_DestroyActor` _output_get))))

(fn `UserConstructionScript`)