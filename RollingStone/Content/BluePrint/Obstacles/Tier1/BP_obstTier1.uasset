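; Tier 1 obstacle that either gets knocked loose or destroys the test actor that runs into it.
; On Collision overlap, it compares its CurrentTierObst2 with that actor's CurrentTier.
; An equal or higher actor tier turns on Cylinder physics, applies the obstacle's own velocity as an impulse, and destroys the obstacle after a delay.
; A lower actor tier destroys the overlapping actor instead.
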(event `self.Collision.OnComponentBeginOverlap`
  (params (OverlappedComponent :type "PrimitiveComponent Object Reference") (OtherActor :type "Actor Object Reference") (OtherComp :type "PrimitiveComponent Object Reference") (OtherBodyIndex :type Integer) (bFromSweep :type Boolean) (SweepResult :type "HitResult Structure (by ref)"))
  (bind _astest (cast `/Game/BluePrint/test` OtherActor))
  (bind _output_get (set `self.As Test_0` _astest))
  (if (<= (`self.currentTierObst2`) (`/Game/BluePrint/test.currentTier` _output_get))
    (`PrimitiveComponent.SetSimulatePhysics` (`self.Cylinder`) true)
    (`PrimitiveComponent.AddImpulse` (`self.Cylinder`) (`self.GetVelocity`) "None" true)
    (`KismetSystemLibrary.Delay` 5.0)
    (`self.K2_DestroyActor`)
    (else
      (`self.K2_DestroyActor` _output_get))))

(fn `UserConstructionScript`)